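; Base building actor for the recycling system, with a coin-priced upgrade state that runs from Level 0 to Level 3.
; On BeginPlay, UpdateRequiredMoneyForBuilding switches on BuildingState to set the next coin cost and enlarge the static mesh from Level 1 upward.
; At Level 3 it applies the largest scale and destroys the UpgradePlatform actor instead of setting a cost.
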(event `self.ReceiveBeginPlay`
  (`self.UpdateRequiredMoneyForBuilding`))

(event `UpdateRequiredMoneyForBuilding`
  (bind _staticmesh (`self.StaticMesh`))
  (switch `/Game/Blueprints/Enums/BuildingState` (`self.BuildingState`)
    (:`NewEnumerator0`
      (set `self.CoinsRequiredToBuy` 5))
    (:`NewEnumerator1`
      (set `self.CoinsRequiredToBuy` 10)
      (`SceneComponent.SetRelativeScale3D` _staticmesh (1.25 1.25 1.25)))
    (:`NewEnumerator2`
      (set `self.CoinsRequiredToBuy` 15)
      (`SceneComponent.SetRelativeScale3D` _staticmesh (1.5 1.5 1.5)))
    (:`NewEnumerator3`
      (`SceneComponent.SetRelativeScale3D` _staticmesh (2.0 2.0 2.0))
      (`self.K2_DestroyActor` (`self.UpgradePlatform`)))))

(fn `UserConstructionScript`)