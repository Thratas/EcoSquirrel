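; ExtractionArea_BP is a trash drop-off zone that empties the player's inventory on overlap and visually cleans up its linked level area.
; Each delivery updates the collected count and widget, and reaching the location maximum disables the LevelBoundsBP box collision.
; A timeline lerps the landscape dynamic material's Pollution parameter, then passes the result to Tree_BP actors inside the level bounds through RiseObject.
; LoadedGame reapplies saved pollution to land and trees without animating the material.
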(event `self.ReceiveBeginPlay`
  (`KismetSystemLibrary.Delay` 0.01)
  (bind _returnvalue (`PrimitiveComponent.CreateDynamicMaterialInstance` (`StaticMeshActor.StaticMeshComponent` (`self.StaticMeshLand`)) 0 "/Game/Environments/Materials/LandscapeInst.LandscapeInst" "None"))
  (set `self.DynamicMaterialLand` _returnvalue)
  (set `self.FoliageInZone` (`self.GetOverlappingActors` (`/Game/Blueprints/Systems/Recycling/LevelBounds_BP.LevelBounds` (`self.LevelBounds_BP`)) "/Game/Blueprints/Systems/Recycling/Tree_BP.Tree_BP_C"))
  (`self.UpdateCollected`))

(event `self.Box.OnComponentBeginOverlap`
  (params (OverlappedComponent :type "PrimitiveComponent Object Reference") (OtherActor :type "Actor Object Reference") (OtherComp :type "PrimitiveComponent Object Reference") (OtherBodyIndex :type Integer) (bFromSweep :type Boolean) (SweepResult :type "HitResult Structure (by ref)"))
  (bind _astop_down_character (cast `/Game/Characters/Player/Blueprints/TopDownCharacter` OtherActor))
  (if (== OtherComp (`Character.CapsuleComponent` _astop_down_character))
    (bind _inventoryarray (`/Game/Characters/Player/Blueprints/TopDownCharacter.InventoryArray` _astop_down_character))
    (for _array_element _inventoryarray
      (message `/Game/Blueprints/Interfaces/Interact.DeliverObject` _array_element)
      (`/Engine/EditorBlueprintResources/StandardMacros.IncrementInt` (`self.CollectedTrash`)))
    (`KismetArrayLibrary.Array_Clear` _inventoryarray)
    (`/Game/Blueprints/Systems/Recycling/LevelBounds_BP.UpdateRemainingTrash` (`self.LevelBounds_BP`))
    (`self.UpdateCollected`)
    (set `/Game/Characters/Player/Blueprints/TopDownCharacter.DesiredSpeed` 600.0 _astop_down_character)))

(event `UpdateCollected`
  (bind _asshow_how_many_collected_wbp (cast `/Game/Core/UI/Widgets/ShowHowManyCollected_WBP` (`WidgetComponent.GetWidget` (`self.ShowHowManyCollectedWidget`))))
  (bind _output_get (set `self.ExtractionData` (make `/Game/Blueprints/Structs/ExtractionData` (`/Game/Blueprints/Systems/Recycling/LevelBounds_BP.MaximumTrashInLocation` (`self.LevelBounds_BP`)) (`self.CollectedTrash`) (`self.CurrentPollution`))))
  (set `/Game/Core/UI/Widgets/ShowHowManyCollected_WBP.Maximum` (break `/Game/Blueprints/Structs/ExtractionData` _output_get) _asshow_how_many_collected_wbp)
  (set `/Game/Core/UI/Widgets/ShowHowManyCollected_WBP.Collected` (`.CollectedTrash_9_611A9C92475CF973D343558EF9ECAA14` (break `/Game/Blueprints/Structs/ExtractionData` _output_get)) _asshow_how_many_collected_wbp)
  (`self.UpdateLand`)
  (if (== (`.CollectedTrash_9_611A9C92475CF973D343558EF9ECAA14` (break `/Game/Blueprints/Structs/ExtractionData` _output_get)) (break `/Game/Blueprints/Structs/ExtractionData` _output_get))
    (`PrimitiveComponent.SetCollisionEnabled` (`/Game/Blueprints/Systems/Recycling/LevelBounds_BP.Box` (`self.LevelBounds_BP`)) "NoCollision")))

(event `UpdateLand`
  (bind (_extractiondata_maximumtrash _extractiondata_collectedtrash) (break `/Game/Blueprints/Structs/ExtractionData` (`self.ExtractionData`)))
  (bind (_maximumtrash _collectedtrash) (break `/Game/Blueprints/Structs/ExtractionData` (`self.ExtractionData`)))
  ;[1 0.4149 0] Pollution Solver -> WIP -> Add function to create flowers etc
  (if (not (`self.IsGameLoading`))
    (set `self.NewPollution` (`KismetMathLibrary.MapRangeClamped` (`KismetMathLibrary.Conv_IntToDouble` _extractiondata_collectedtrash) 0.0 (`KismetMathLibrary.Conv_IntToDouble` _extractiondata_maximumtrash) 1.0))
    (bind (_direction _newtrack_0) (`Timeline|Timeline_0` :!via `PlayFromStart`)
      (:`Update`
        (bind _dynamicmaterialland (`self.DynamicMaterialLand`)
          (:`then`
            (bind _returnvalue (`KismetMathLibrary.Lerp` (`self.CurrentPollution`) (`self.NewPollution`) _newtrack_0))
            (`MaterialInstanceDynamic.SetScalarParameterValue` _dynamicmaterialland "Pollution" _returnvalue))
          (:`else`)))
      (:`Finished`
        (set `self.CurrentPollution` _returnvalue)
        (set `self.ExtractionData` (make `/Game/Blueprints/Structs/ExtractionData` _maximumtrash _collectedtrash (`self.CurrentPollution`)))
        (for _array_element (`self.FoliageInZone`)
          (bind _astree_bp (cast `/Game/Blueprints/Systems/Recycling/Tree_BP` _array_element))
          (`/Game/Blueprints/Systems/Recycling/Tree_BP.RiseObject` _astree_bp (`.CurrentPollution_4_92C6E36D45696C444B28D3ADF41E9637` (break `/Game/Blueprints/Structs/ExtractionData` (`self.ExtractionData`))) false))))))

(event `LoadedGame`
  (set `self.IsGameLoading` true)
  (`KismetSystemLibrary.Delay` 0.01)
  (bind _dynamicmaterialland (`self.DynamicMaterialLand`)
    (:`then`
      (`MaterialInstanceDynamic.SetScalarParameterValue` _dynamicmaterialland "Pollution" (`.CurrentPollution_4_92C6E36D45696C444B28D3ADF41E9637` (break `/Game/Blueprints/Structs/ExtractionData` (`self.ExtractionData`))))
      (for _array_element (`self.FoliageInZone`)
        (bind _astree_bp (cast `/Game/Blueprints/Systems/Recycling/Tree_BP` _array_element))
        (`/Game/Blueprints/Systems/Recycling/Tree_BP.RiseObject` _astree_bp (`.CurrentPollution_4_92C6E36D45696C444B28D3ADF41E9637` (break `/Game/Blueprints/Structs/ExtractionData` (`self.ExtractionData`))) true))
      (`KismetSystemLibrary.Delay` 0.2)
      (set `self.IsGameLoading` false))
    (:`else`)))

(fn `UserConstructionScript`)