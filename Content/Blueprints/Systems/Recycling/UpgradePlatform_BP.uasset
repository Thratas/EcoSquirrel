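; UpgradePlatform is an interactable pad that lets the player spend AcornMoney to upgrade its linked BuildingBase.
; Its Box overlap sets or clears the player's TargetToPickUp, using a player reference cached on BeginPlay.
; On Interact, it checks the building's cost, advances BuildingState one level up to Level3, deducts the money and has the building update its required money.
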(event `self.ReceiveBeginPlay`
  (bind _astop_down_character (cast `/Game/Characters/Player/Blueprints/TopDownCharacter` (`GameplayStatics.GetPlayerPawn` 0)))
  (set `self.PlayerRef` _astop_down_character))

(event `self.Box.OnComponentBeginOverlap`
  (params (OverlappedComponent :type "PrimitiveComponent Object Reference") (OtherActor :type "Actor Object Reference") (OtherComp :type "PrimitiveComponent Object Reference") (OtherBodyIndex :type Integer) (bFromSweep :type Boolean) (SweepResult :type "HitResult Structure (by ref)"))
  (if (== OtherComp (`Character.CapsuleComponent` (`self.PlayerRef`)))
    (set `/Game/Characters/Player/Blueprints/TopDownCharacter.TargetToPickUp` self (`self.PlayerRef`))))

(event `self.Box.OnComponentEndOverlap`
  (params (OverlappedComponent :type "PrimitiveComponent Object Reference") (OtherActor :type "Actor Object Reference") (OtherComp :type "PrimitiveComponent Object Reference") (OtherBodyIndex :type Integer))
  (if (== OtherComp (`Character.CapsuleComponent` (`self.PlayerRef`)))
    (set `/Game/Characters/Player/Blueprints/TopDownCharacter.TargetToPickUp` null (`self.PlayerRef`))))

(event `/Game/Blueprints/Interfaces/Interact.Interact`
  (switch `/Game/Blueprints/Enums/BuildingState` (`/Game/Blueprints/Systems/Recycling/Building_Base_BP.BuildingState` (`self.BuildingBase`))
    (:`NewEnumerator0`
      (if (>= (`/Game/Characters/Player/Blueprints/TopDownCharacter.AcornMoney` (`self.PlayerRef`)) (`/Game/Blueprints/Systems/Recycling/Building_Base_BP.CoinsRequiredToBuy` (`self.BuildingBase`)))
        (set `/Game/Blueprints/Systems/Recycling/Building_Base_BP.BuildingState` "NewEnumerator1" (`self.BuildingBase`))
        (set `/Game/Characters/Player/Blueprints/TopDownCharacter.AcornMoney` (- (`/Game/Characters/Player/Blueprints/TopDownCharacter.AcornMoney` (`self.PlayerRef`)) (`/Game/Blueprints/Systems/Recycling/Building_Base_BP.CoinsRequiredToBuy` (`self.BuildingBase`))) (`self.PlayerRef`))
        (`/Game/Blueprints/Systems/Recycling/Building_Base_BP.UpdateRequiredMoneyForBuilding` (`self.BuildingBase`))))
    (:`NewEnumerator1`
      (if (>= (`/Game/Characters/Player/Blueprints/TopDownCharacter.AcornMoney` (`self.PlayerRef`)) (`/Game/Blueprints/Systems/Recycling/Building_Base_BP.CoinsRequiredToBuy` (`self.BuildingBase`)))
        (set `/Game/Blueprints/Systems/Recycling/Building_Base_BP.BuildingState` "NewEnumerator2" (`self.BuildingBase`))
        (set `/Game/Characters/Player/Blueprints/TopDownCharacter.AcornMoney` (- (`/Game/Characters/Player/Blueprints/TopDownCharacter.AcornMoney` (`self.PlayerRef`)) (`/Game/Blueprints/Systems/Recycling/Building_Base_BP.CoinsRequiredToBuy` (`self.BuildingBase`))) (`self.PlayerRef`))
        (`/Game/Blueprints/Systems/Recycling/Building_Base_BP.UpdateRequiredMoneyForBuilding` (`self.BuildingBase`))))
    (:`NewEnumerator2`
      (if (>= (`/Game/Characters/Player/Blueprints/TopDownCharacter.AcornMoney` (`self.PlayerRef`)) (`/Game/Blueprints/Systems/Recycling/Building_Base_BP.CoinsRequiredToBuy` (`self.BuildingBase`)))
        (set `/Game/Blueprints/Systems/Recycling/Building_Base_BP.BuildingState` "NewEnumerator3" (`self.BuildingBase`))
        (set `/Game/Characters/Player/Blueprints/TopDownCharacter.AcornMoney` (- (`/Game/Characters/Player/Blueprints/TopDownCharacter.AcornMoney` (`self.PlayerRef`)) (`/Game/Blueprints/Systems/Recycling/Building_Base_BP.CoinsRequiredToBuy` (`self.BuildingBase`))) (`self.PlayerRef`))
        (`/Game/Blueprints/Systems/Recycling/Building_Base_BP.UpdateRequiredMoneyForBuilding` (`self.BuildingBase`))))))

(fn `UserConstructionScript`)