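; Tree actor for the recycling system that emerges from the ground as pollution drops.
; On BeginPlay it picks a random mesh from an array for its static mesh.
; RiseObject fires once when current pollution is at or below its required threshold, then either snaps the mesh to its raised position for loaded games or plays a timeline lerping it upward.
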(event `self.ReceiveBeginPlay`
  (bind _output_get (set `self.StaticMeshToSelect` (`KismetArrayLibrary.Array_Random` (`self.ArrayOfMeshes`))))
  (`StaticMeshComponent.SetStaticMesh` (`self.StaticMesh`) _output_get))

(event `RiseObject`
  (params (CurrentPollution :type "Float (double-precision)") (GameLoaded :type Boolean))
  (bind _staticmesh (`self.StaticMesh`))
  (if (<= CurrentPollution (`self.PollutionProgressRequired`))
    (`/Engine/EditorBlueprintResources/StandardMacros.DoOnce` false
      (:`Completed`
        (if GameLoaded
          (`SceneComponent.K2_SetRelativeLocation` _staticmesh (0.0 0.0 150.0) false false)
          (else
            (bind (_direction _newtrack_0) (`Timeline|RiseUp` :!via `PlayFromStart`)
              (:`Update`
                (`SceneComponent.K2_SetRelativeLocation` _staticmesh (`KismetMathLibrary.VLerp` (0.0 0.0 -220.0) (0.0 0.0 150.0) _newtrack_0) false false)))))))))

(fn `UserConstructionScript`)